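; AI controller for NPCs that starts the Patrol behavior tree on the PatrolData blackboard at BeginPlay.
; AI perception updates only print a debug string naming the pawn, sense class and detected actor.
; GetPatrol writes the controlled ThirdPersonCharacter's first patrol point to the Waypoint key, but its call in the event graph is disconnected and never runs.
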(event `self.ReceiveBeginPlay`
  (`self.UseBlackboard` "/Game/Blueprints/PatrolData.PatrolData")
  (`self.RunBehaviorTree` "/Game/Blueprints/Patrol.Patrol"))

(event `self.AIPerception.OnTargetPerceptionUpdated`
  (params (Actor :type "Actor Object Reference") (Stimulus :type "AIStimulus Structure"))
  (bind _returnvalue (`AIPerceptionSystem.GetSenseClassForStimulus` Stimulus))
  (`KismetSystemLibrary.PrintString` (`KismetStringLibrary.Concat_StrStr` (`KismetSystemLibrary.GetObjectName` (`self.K2_GetPawn`)) " " (`KismetSystemLibrary.GetClassDisplayName` _returnvalue) " " (`KismetSystemLibrary.GetObjectName` Actor))))

(fn `GetPatrol`
  (params (blackBoard :type "BlackboardComponent Object Reference"))
  (bind _asthird_person_character (cast `/Game/ThirdPersonCPP/Blueprints/ThirdPersonCharacter` (`self.K2_GetPawn`)))
  (`BlackboardComponent.SetValueAsObject` blackBoard "Waypoint" (`|GetArrayItem` (`/Game/ThirdPersonCPP/Blueprints/ThirdPersonCharacter.PatrolPoints` _asthird_person_character))))

(fn `UserConstructionScript`)